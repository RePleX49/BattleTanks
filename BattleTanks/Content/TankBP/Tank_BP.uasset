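; Tank pawn Blueprint that sets up camera look input and registers its barrel component.
; On BeginPlay the InputSetup graph passes the Barrel to SetBarrelReference.
; Turn and LookUp axes feed controller yaw and pitch directly, while TurnRate and LookUpRate scale by rate and delta seconds for frame-independent turning.
; Turn and LookUp handlers appear in both EventGraph and InputSetup.
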(event `InputAxis|LookUp`
  (params (AxisValue :type "Float (single-precision)"))
  (`self.AddControllerPitchInput` AxisValue))

(event `InputAxis|Turn`
  (params (AxisValue :type "Float (single-precision)"))
  (`self.AddControllerYawInput` AxisValue))

(event `self.ReceiveBeginPlay`
  (`self.SetBarrelReference` (`self.Barrel`)))

(event `InputAxis|Turn`
  (params (AxisValue :type "Float (single-precision)"))
  (`self.AddControllerYawInput` AxisValue))

(event `InputAxis|LookUp`
  (params (AxisValue :type "Float (single-precision)"))
  (`self.AddControllerPitchInput` AxisValue))

(event `InputAxis|TurnRate`
  (params (AxisValue :type "Float (single-precision)"))
  (`self.AddControllerYawInput` (* AxisValue (`self.TurnRate`) (`GameplayStatics.GetWorldDeltaSeconds`))))

(event `InputAxis|LookUpRate`
  (params (AxisValue :type "Float (single-precision)"))
  (`self.AddControllerPitchInput` (* AxisValue (`self.LookUpRate`) (`GameplayStatics.GetWorldDeltaSeconds`))))

(fn `UserConstructionScript`)