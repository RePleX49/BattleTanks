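; EnergySource is a Blueprint that traces a straight beam from its BeamSourcePoint component.
; On BeginPlay, a looping timer calls EmitBeam ten times a second to line trace a short fixed distance forward on the Visibility channel.
; It stores the source position and hit location as BeamStart and BeamEnd, without checking for a hit.
; The only visual in the graph is the trace's persistent debug drawing.
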(event `self.ReceiveBeginPlay`
  (`KismetSystemLibrary.K2_SetTimerDelegate` (delegate `EmitBeam`) 0.1 true))

(event `EmitBeam`
  (bind _beamsourcepoint (`self.BeamSourcePoint`))
  (bind _returnvalue (`SceneComponent.K2_GetComponentLocation` _beamsourcepoint))
  (set `self.BeamStart` _returnvalue)
  (bind _outhit (`KismetSystemLibrary.LineTraceSingle` :`Start` _returnvalue :`End` (+ _returnvalue (* (`SceneComponent.GetForwardVector` _beamsourcepoint) 500.0)) :`TraceChannel` "TraceTypeQuery1" :`DrawDebugType` "Persistent"))
  (set `self.BeamEnd` (`.Location` (`GameplayStatics.BreakHitResult` _outhit))))

(fn `UserConstructionScript`)